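; BP_GoToCinemaDoor is a door, named as the way to the cinema, that swings open automatically when a Character enters its interaction volume.
; The Open timeline lerps the door's relative yaw on overlap and reverses when the Character leaves.
; The same overlaps set an IsOpen flag and toggle a text block in the interaction widget, reached through the cached BP_MainPlatformGamemode.
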(event OnComponentBeginOverlap(Door_Interaction)
  (params (OverlappedComponent :type Primitive%20Component%20Object%20Reference) (OtherActor :type Actor%20Object%20Reference) (OtherComp :type Primitive%20Component%20Object%20Reference) (OtherBodyIndex :type Integer) (bFromSweep :type Boolean) (SweepResult :type Hit%20Result%20Structure%20%28by%20ref%29))
  (Utilities|Casting|CastToCharacter OtherActor)
  (Variables|Default|SetIsOpen true)
  (Widget|SetVisibility (Variables|/Game/CHJ/Widgets/WBP_InteractionWidget.WBP_InteractionWidget_C|GetTextBlock_36 (Variables|/Game/CHJ/Widgets/WBP_MainPlatformWidget.WBP_MainPlatformWidget_C|GetWBP_InteractionWidget (Variables|/Game/CHJ/BP_MainPlatformGamemode.BP_MainPlatformGamemode_C|GetWidget (Variables|Default|GetGameMode)))) "Visible")
  (bind _kick (Timeline|Open Play)
    (:Update
      (Transformation|SetRelativeRotation (Variables|Default|GetDoor) (Math|Rotator|MakeRotator 0.0 0.0 (Math|Float|Lerp 0.0 -1.2e+02 _kick)) false false))))

(event OnComponentEndOverlap(Door_Interaction)
  (params (OverlappedComponent :type Primitive%20Component%20Object%20Reference) (OtherActor :type Actor%20Object%20Reference) (OtherComp :type Primitive%20Component%20Object%20Reference) (OtherBodyIndex :type Integer))
  (Utilities|Casting|CastToCharacter OtherActor)
  (Variables|Default|SetIsOpen false)
  (Widget|SetVisibility (Variables|/Game/CHJ/Widgets/WBP_InteractionWidget.WBP_InteractionWidget_C|GetTextBlock_36 (Variables|/Game/CHJ/Widgets/WBP_MainPlatformWidget.WBP_MainPlatformWidget_C|GetWBP_InteractionWidget (Variables|/Game/CHJ/BP_MainPlatformGamemode.BP_MainPlatformGamemode_C|GetWidget (Variables|Default|GetGameMode)))) "Hidden")
  (bind _kick (Timeline|Open Reverse)
    (:Update
      (Transformation|SetRelativeRotation (Variables|Default|GetDoor) (Math|Rotator|MakeRotator 0.0 0.0 (Math|Float|Lerp 0.0 -1.2e+02 _kick)) false false))))

(event EventBeginPlay
  (bind _asbp_main_platform_gamemode (Utilities|Casting|CastToBP_MainPlatformGamemode (Game|GetGameMode)))
  (Variables|Default|SetGameMode _asbp_main_platform_gamemode))

(fn ConstructionScript)