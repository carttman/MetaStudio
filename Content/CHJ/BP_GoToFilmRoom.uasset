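; A clickable actor that switches the main platform UI to another page, named for going to the film room.
; On BeginPlay it enables click events on the player controller and caches the main platform game mode.
; Clicking its box, confirmed by a visibility trace under the cursor, marks it clicked, sets the game mode widget's switcher to a fixed page, and disables further click events.
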(event OnClicked(Box)
  (params (TouchedComponent :type Primitive%20Component%20Object%20Reference) (ButtonPressed :type Key%20Structure :default "None"))
  (if (.ReturnValue (Game|Player|GetHitResultUnderCursorbyChannel (Game|GetPlayerController 0) "TraceTypeQuery1" true))
    (Variables|Default|SetbIsClicked true)
    (Variables|/Script/UMG.WidgetSwitcher|SetActiveWidgetIndex (Variables|/Game/CHJ/Widgets/WBP_MainPlatformWidget.WBP_MainPlatformWidget_C|GetWS_MainPlatfromSwitcher (Variables|/Game/CHJ/GameMode/BP_MainPlatformGamemode.BP_MainPlatformGamemode_C|GetWidget (Variables|Default|GetGameMode))) 2)
    (Variables|/Script/Engine.PlayerController|SetbEnableClickEvents (Game|GetPlayerController 0) false)))

(event EventBeginPlay
  (Variables|/Script/Engine.PlayerController|SetbEnableClickEvents (Game|GetPlayerController 0) true)
  (bind _asbp_main_platform_gamemode (Utilities|Casting|CastToBP_MainPlatformGamemode (Game|GetGameMode)))
  (Variables|Default|SetGameMode _asbp_main_platform_gamemode))

(event Collision|EventActorBeginOverlap
  (params (OtherActor :type Actor%20Object%20Reference)))

(event EventTick
  (params (DeltaSeconds :type Float%20%28single-precision%29)))

(fn ConstructionScript)