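; BP_GoToCinema is a trigger actor that sends the game to the cinema lobby level.
; Any Character overlapping its Box opens CinemaLobbyMap by object reference, with no check that it is the player.
; Each Tick, its Widget rotates along the line from the player character cached at BeginPlay, applying that world-space direction as relative rotation with X pointing away from the player.
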(event OnComponentBeginOverlap(Box)
  (params (OverlappedComponent :type Primitive%20Component%20Object%20Reference) (OtherActor :type Actor%20Object%20Reference) (OtherComp :type Primitive%20Component%20Object%20Reference) (OtherBodyIndex :type Integer) (bFromSweep :type Boolean) (SweepResult :type Hit%20Result%20Structure%20%28by%20ref%29))
  (Utilities|Casting|CastToCharacter OtherActor)
  (Game|OpenLevel(byObjectReference) "/Game/Maps/CinemaLobbyMap.CinemaLobbyMap"))

(event EventBeginPlay
  (bind _ascharacter (Utilities|Casting|CastToCharacter (Game|Player|GetPlayerPawn 0)))
  (Variables|Default|SetCharacter _ascharacter))

(event Collision|EventActorBeginOverlap
  (params (OtherActor :type Actor%20Object%20Reference)))

(event EventTick
  (params (DeltaSeconds :type Float%20%28single-precision%29))
  (Transformation|SetRelativeRotation (Variables|Default|GetWidget) (Math|Conversions|RotationFromXVector (Math|Vector|Normalize (- (Transformation|GetWorldLocation (Variables|Default|GetWidget)) (Transformation|GetActorLocation (Variables|Default|GetCharacter))))) false false))

(fn ConstructionScript)