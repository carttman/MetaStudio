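; BP_MainPlatformCharacter is the main platform character, handling the F key interaction at the cinema and film room doors.
; It caches BP_MainPlatformGamemode on BeginPlay to reach that game mode's widget.
; Pressing F finds each door actor by class and, if its IsOpen is set, switches the widget switcher to that door's panel and shows the mouse cursor.
; Direct level-open nodes for both lobby maps remain unconnected.
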(event EventBeginPlay
  (|CallParentFunction)
  (bind _asbp_main_platform_gamemode (Utilities|Casting|CastToBP_MainPlatformGamemode (Game|GetGameMode)))
  (Variables|Default|SetGameMode _asbp_main_platform_gamemode))

(event Collision|EventActorBeginOverlap
  (params (OtherActor :type Actor%20Object%20Reference))
  (|CallParentFunction OtherActor) ; This node is disabled and will not be called.\nDrag off pins to build functionality.
)

(event EventTick
  (params (DeltaSeconds :type Float%20%28single-precision%29))
  (|CallParentFunction DeltaSeconds) ; This node is disabled and will not be called.\nDrag off pins to build functionality.
)

(event Input|KeyboardEvents|F
  (params (Key :type Key%20Structure))
  (bind _returnvalue (Game|GetPlayerController 0))
  (bind _gamemode (Variables|Default|GetGameMode))
  (bind _widget (Variables|/Game/CHJ/BP_MainPlatformGamemode.BP_MainPlatformGamemode_C|GetWidget _gamemode))
  (bind _ws_mainplatfromswitcher (Variables|/Game/CHJ/Widgets/WBP_MainPlatformWidget.WBP_MainPlatformWidget_C|GetWS_MainPlatfromSwitcher _widget))
  (:Pressed
    (Utilities|FlowControl|Sequence
      (:then_0
        (bind _returnvalue_2 (Actor|GetActorOfClass "/Game/CHJ/Door/BP_GoToCinemaDoor.BP_GoToCinemaDoor_C"))
        (if (Variables|/Game/CHJ/Door/BP_GoToCinemaDoor.BP_GoToCinemaDoor_C|GetIsOpen _returnvalue_2)
          (Class|WidgetSwitcher|SetActiveWidgetIndex _ws_mainplatfromswitcher 1)
          (Variables|/Script/Engine.PlayerController|SetbShowMouseCursor _returnvalue true)))
      (:then_1
        (bind _returnvalue_3 (Actor|GetActorOfClass "/Game/CHJ/Door/BP_GoToFilmRoomDoor.BP_GoToFilmRoomDoor_C"))
        (if (Variables|/Game/CHJ/Door/BP_GoToFilmRoomDoor.BP_GoToFilmRoomDoor_C|GetIsOpen _returnvalue_3)
          (Class|WidgetSwitcher|SetActiveWidgetIndex _ws_mainplatfromswitcher 2)
          (Variables|/Script/Engine.PlayerController|SetbShowMouseCursor _returnvalue true))))))

(fn ConstructionScript
  (|CallParentFunction))