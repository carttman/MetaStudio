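; BP_GoToFilm is a clickable slate in the main lobby that moves the camera to the film view.
; Hovering its Box plays the board animation; clicking uses a Timeline to lerp the lobby cine camera to Point, then switches the game mode widget's switcher to index 1.
; FilmRoomEvent reverses this, restoring index 0 and easing the camera back to the camera actor's Arrow.
; BeginPlay enables mouse events and caches the game mode and camera.
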(event OnEndCursorOver(Box)
  (params (TouchedComponent :type Primitive%20Component%20Object%20Reference)))

(event OnClicked(Box)
  (params (TouchedComponent :type Primitive%20Component%20Object%20Reference) (ButtonPressed :type Key%20Structure :default "None"))
  (bind _mainlobbycamera (Variables|Default|GetMainLobbyCamera))
  (bind _cinecamera (Variables|/Game/CHJ/BP_MainLobbyCamera.BP_MainLobbyCamera_C|GetCineCamera _mainlobbycamera))
  (if (.ReturnValue (Game|Player|GetHitResultUnderCursorbyChannel (Game|GetPlayerController 0) "TraceTypeQuery1" true))
    (Variables|Default|SetbIsClicked true)
    (bind _move (Timeline|Timeline PlayFromStart)
      (:Update
        (Transformation|SetWorldLocation _cinecamera (Math|Vector|Lerp(Vector) (Transformation|GetWorldLocation _cinecamera) (Transformation|GetWorldLocation (Variables|Default|GetPoint)) _move) false false))
      (:Finished
        (Variables|/Script/UMG.WidgetSwitcher|SetActiveWidgetIndex (Variables|/Game/CHJ/Widgets/WBP_MainPlatformWidget.WBP_MainPlatformWidget_C|GetWS_MainPlatfromSwitcher (Variables|/Game/CHJ/GameMode/BP_MainPlatformGamemode.BP_MainPlatformGamemode_C|GetWidget (Variables|Default|GetGameMode))) 1)))))

(event OnBeginCursorOver(Box)
  (params (TouchedComponent :type Primitive%20Component%20Object%20Reference))
  (Components|Animation|PlayAnimation (Variables|Default|GetSlate) "/Game/SYM/3Dasset/Board/board_Anim.board_Anim" false))

(event Custom|FilmRoomEvent
  (bind _mainlobbycamera (Variables|Default|GetMainLobbyCamera))
  (bind _cinecamera (Variables|/Game/CHJ/BP_MainLobbyCamera.BP_MainLobbyCamera_C|GetCineCamera _mainlobbycamera))
  (Variables|/Script/UMG.WidgetSwitcher|SetActiveWidgetIndex (Variables|/Game/CHJ/Widgets/WBP_MainPlatformWidget.WBP_MainPlatformWidget_C|GetWS_MainPlatfromSwitcher (Variables|/Game/CHJ/GameMode/BP_MainPlatformGamemode.BP_MainPlatformGamemode_C|GetWidget (Variables|Default|GetGameMode))) 0)
  (bind _move (Timeline|Timeline_0 PlayFromStart)
    (:Update
      (Transformation|SetWorldLocation _cinecamera (Math|Vector|Lerp(Vector) (Transformation|GetWorldLocation _cinecamera) (Transformation|GetWorldLocation (Variables|/Game/CHJ/BP_MainLobbyCamera.BP_MainLobbyCamera_C|GetArrow _mainlobbycamera)) _move) false false))))

(event EventBeginPlay
  (bind _returnvalue (Game|GetPlayerController 0))
  (Variables|/Script/Engine.PlayerController|SetbEnableClickEvents _returnvalue true)
  (Variables|/Script/Engine.PlayerController|SetbEnableMouseOverEvents _returnvalue true)
  (bind _asbp_main_platform_gamemode (Utilities|Casting|CastToBP_MainPlatformGamemode (Game|GetGameMode)))
  (Variables|Default|SetGameMode _asbp_main_platform_gamemode)
  (bind _returnvalue_2 (Actor|GetActorOfClass "/Game/CHJ/BP_MainLobbyCamera.BP_MainLobbyCamera_C"))
  (Variables|Default|SetMainLobbyCamera _returnvalue_2))

(event Collision|EventActorBeginOverlap
  (params (OtherActor :type Actor%20Object%20Reference)))

(event EventTick
  (params (DeltaSeconds :type Float%20%28single-precision%29)))

(fn ConstructionScript)