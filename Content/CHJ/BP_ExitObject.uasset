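; Clickable exit actor, apparently for the main lobby, that quits the game when its Box is clicked.
; BeginPlay enables mouse click and hover events on the player controller, caches BP_MainPlatformGamemode and shows the Widget component's UI.
; Cursor hover on the Box tints that widget red-orange and restores white on leave.
; Disconnected leftover logic for visibility toggles, a lobby camera timeline move and menu switching never runs.
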(event OnEndCursorOver(Box)
  (params (TouchedComponent :type Primitive%20Component%20Object%20Reference))
  (Appearance|SetColorandOpacity (UserInterface|GetUserWidgetObject (Variables|Default|GetWidget)) "(R=1.000000,G=1.000000,B=1.000000,A=1.000000)" :!class /Script/UMG.UserWidget))

(event OnClicked(Box)
  (params (TouchedComponent :type Primitive%20Component%20Object%20Reference) (ButtonPressed :type Key%20Structure :default "None"))
  (Game|QuitGame 0 "Quit" false))

(event OnBeginCursorOver(Box)
  (params (TouchedComponent :type Primitive%20Component%20Object%20Reference))
  (Appearance|SetColorandOpacity (UserInterface|GetUserWidgetObject (Variables|Default|GetWidget)) "(R=1.000000,G=0.319591,B=0.226505,A=1.000000)" :!class /Script/UMG.UserWidget))

(event EventBeginPlay
  (bind _returnvalue (Game|GetPlayerController 0))
  (Variables|/Script/Engine.PlayerController|SetbEnableClickEvents _returnvalue true)
  (Variables|/Script/Engine.PlayerController|SetbEnableMouseOverEvents _returnvalue true)
  (bind _asbp_main_platform_gamemode (Utilities|Casting|CastToBP_MainPlatformGamemode (Game|GetGameMode)))
  (Variables|Default|SetGameMode _asbp_main_platform_gamemode)
  (Widget|SetVisibility (UserInterface|GetUserWidgetObject (Variables|Default|GetWidget)) "Visible"))

(event Collision|EventActorBeginOverlap
  (params (OtherActor :type Actor%20Object%20Reference)))

(event EventTick
  (params (DeltaSeconds :type Float%20%28single-precision%29)))

(fn ConstructionScript)