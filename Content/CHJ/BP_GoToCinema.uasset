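; Clickable lobby hotspot that takes the player into the cinema section of the main platform UI.
; Hovering its Box reveals a widget and spawns a popcorn effect.
; Clicking runs a Timeline that lerps the lobby cine camera to Point, then switches the gamemode's widget switcher page and blurs the background.
; CinemaEvent reverses this, clearing the blur, restoring the first page and easing the camera back to its Arrow.
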(event OnBeginCursorOver(Box)
  (params (TouchedComponent :type Primitive%20Component%20Object%20Reference))
  (bind _effectpoint_0 (Variables|Default|GetEffectPoint_0))
  (bind _returnvalue (Niagara|SpawnSystematLocation (Variables|Default|GetPopcornVFX) (Transformation|GetWorldLocation _effectpoint_0) (Transformation|GetWorldRotation _effectpoint_0)))
  (Widget|SetVisibility (UserInterface|GetUserWidgetObject (Variables|Default|GetWidget)) "Visible"))

(event OnClicked(Box)
  (params (TouchedComponent :type Primitive%20Component%20Object%20Reference) (ButtonPressed :type Key%20Structure :default "None"))
  (bind _gamemode (Variables|Default|GetGameMode))
  (bind _mainlobbycamera (Variables|Default|GetMainLobbyCamera))
  (bind _widget (Variables|/Game/CHJ/GameMode/BP_MainPlatformGamemode.BP_MainPlatformGamemode_C|GetWidget _gamemode))
  (bind _cinecamera (Variables|/Game/CHJ/BP_MainLobbyCamera.BP_MainLobbyCamera_C|GetCineCamera _mainlobbycamera))
  (if (.ReturnValue (Game|Player|GetHitResultUnderCursorbyChannel (Game|GetPlayerController 0) "TraceTypeQuery1" true))
    (bind _move (Timeline|Timeline PlayFromStart)
      (:Update
        (Transformation|SetWorldLocation _cinecamera (Math|Vector|Lerp(Vector) (Transformation|GetWorldLocation _cinecamera) (Transformation|GetWorldLocation (Variables|Default|GetPoint)) _move) false false))
      (:Finished
        (Variables|/Script/UMG.WidgetSwitcher|SetActiveWidgetIndex (Variables|/Game/CHJ/Widgets/WBP_MainPlatformWidget.WBP_MainPlatformWidget_C|GetWS_MainPlatfromSwitcher _widget) 2)
        (Class|BackgroundBlur|SetBlurStrength (Variables|/Game/CHJ/Widgets/WBP_MainPlatformWidget.WBP_MainPlatformWidget_C|GetBG_Blur _widget) 5.0)))))

(event OnEndCursorOver(Box)
  (params (TouchedComponent :type Primitive%20Component%20Object%20Reference))
  (Components|Activation|Deactivate (stale OnBeginCursorOver(Box) _returnvalue))
  (Widget|SetVisibility (UserInterface|GetUserWidgetObject (Variables|Default|GetWidget)) "Hidden"))

(event Custom|CinemaEvent
  (bind _mainlobbycamera (Variables|Default|GetMainLobbyCamera))
  (bind _gamemode (Variables|Default|GetGameMode))
  (bind _cinecamera (Variables|/Game/CHJ/BP_MainLobbyCamera.BP_MainLobbyCamera_C|GetCineCamera _mainlobbycamera))
  (bind _widget (Variables|/Game/CHJ/GameMode/BP_MainPlatformGamemode.BP_MainPlatformGamemode_C|GetWidget _gamemode))
  (Class|BackgroundBlur|SetBlurStrength (Variables|/Game/CHJ/Widgets/WBP_MainPlatformWidget.WBP_MainPlatformWidget_C|GetBG_Blur _widget) 0.0)
  (Variables|/Script/UMG.WidgetSwitcher|SetActiveWidgetIndex (Variables|/Game/CHJ/Widgets/WBP_MainPlatformWidget.WBP_MainPlatformWidget_C|GetWS_MainPlatfromSwitcher _widget) 0)
  (bind _move (Timeline|Timeline_0 PlayFromStart)
    (:Update
      (Transformation|SetWorldLocation _cinecamera (Math|Vector|Lerp(Vector) (Transformation|GetWorldLocation _cinecamera) (Transformation|GetWorldLocation (Variables|/Game/CHJ/BP_MainLobbyCamera.BP_MainLobbyCamera_C|GetArrow _mainlobbycamera)) _move) false false))))

(event EventBeginPlay
  (bind _returnvalue (Game|GetPlayerController 0))
  (Variables|/Script/Engine.PlayerController|SetbEnableClickEvents _returnvalue true)
  (Variables|/Script/Engine.PlayerController|SetbEnableMouseOverEvents _returnvalue true)
  (bind _asbp_main_platform_gamemode (Utilities|Casting|CastToBP_MainPlatformGamemode (Game|GetGameMode)))
  (Variables|Default|SetGameMode _asbp_main_platform_gamemode)
  (bind _returnvalue_2 (Actor|GetActorOfClass "/Game/CHJ/BP_MainLobbyCamera.BP_MainLobbyCamera_C"))
  (Variables|Default|SetMainLobbyCamera _returnvalue_2)
  (Widget|SetVisibility (UserInterface|GetUserWidgetObject (Variables|Default|GetWidget)) "Hidden"))

(event Collision|EventActorBeginOverlap
  (params (OtherActor :type Actor%20Object%20Reference)))

(event EventTick
  (params (DeltaSeconds :type Float%20%28single-precision%29)))

(fn ConstructionScript)