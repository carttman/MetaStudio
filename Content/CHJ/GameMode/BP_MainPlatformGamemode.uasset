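; BP_MainPlatformGamemode is the game mode for the main platform, setting up its UI and the hook from the film room lobby to the cinema actor.
; On BeginPlay it shows the mouse cursor, adds WBP_MainPlatformWidget to the viewport and binds the nested film room lobby's FSButtonGoMenu click.
; That click looks up the BP_GoToCinema actor by class and calls its function named 123.
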(event Custom|MyOnClicked
  (bind _returnvalue (Actor|GetActorOfClass "/Game/CHJ/BP_GoToCinema.BP_GoToCinema_C"))
  (Default|123 _returnvalue))

(event EventBeginPlay
  (Variables|/Script/Engine.PlayerController|SetbShowMouseCursor (Game|GetPlayerController 0) true)
  (bind _returnvalue (UserInterface|CreateWidget "/Game/CHJ/Widgets/WBP_MainPlatformWidget.WBP_MainPlatformWidget_C"))
  (bind _output_get (Variables|Default|SetWidget _returnvalue))
  (UserInterface|Viewport|AddtoViewport _output_get 0)
  (EventDispatchers|BindEventtoOnClicked (Variables|/Script/MetaStudios.FilmRoomLobbyWidget|GetFS_Button_GoMenu (Variables|/Game/CHJ/Widgets/WBP_MainPlatformWidget.WBP_MainPlatformWidget_C|GetWBP_FilmRoomLobbyWidget _output_get)) (delegate Custom|MyOnClicked)))

(event EventTick
  (params (DeltaSeconds :type Float%20%28single-precision%29)))

(fn ConstructionScript)