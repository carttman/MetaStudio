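; An interaction door Blueprint for a kick action, apparently unfinished, with debug prints throughout.
; The ckic, SKIC and MKick events chain into a DoOnce that snaps the actor's transform to its SkeletalMesh's world transform.
; The Door_Interaction overlap events are empty.
; The Kick timeline that swings the Door on yaw, the KickDoor flag and the gate logic are disconnected and never run.
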(event OnComponentBeginOverlap(Door_Interaction)
  (params (OverlappedComponent :type Primitive%20Component%20Object%20Reference) (OtherActor :type Actor%20Object%20Reference) (OtherComp :type Primitive%20Component%20Object%20Reference) (OtherBodyIndex :type Integer) (bFromSweep :type Boolean) (SweepResult :type Hit%20Result%20Structure%20%28by%20ref%29)))

(event OnComponentEndOverlap(Door_Interaction)
  (params (OverlappedComponent :type Primitive%20Component%20Object%20Reference) (OtherActor :type Actor%20Object%20Reference) (OtherComp :type Primitive%20Component%20Object%20Reference) (OtherBodyIndex :type Integer)))

(event Custom|MKick
  (Development|PrintString "3")
  (Utilities|FlowControl|Sequence
    (:then_0
      (Utilities|FlowControl|DoOnce false
        (:Completed
          (Development|PrintString "4")
          (Transformation|SetActorTransform (Transformation|GetWorldTransform (Variables|Default|GetSkeletalMesh)))
          (Development|PrintString "5"))))))

(event Custom|SKIC
  (Utilities|FlowControl|Sequence
    (:then_1
      (Development|PrintString "44H2")
      (CallFunction|MKick)
      (Development|PrintString "H2"))))

(event Custom|ckic
  (CallFunction|SKIC)
  (Development|PrintString "Hello2")
  (CallFunction|MKick)
  (Utilities|FlowControl|Sequence
    (:then_0
      (Utilities|FlowControl|DoOnce false
        (:Completed
          (Development|PrintString "4")
          (Transformation|SetActorTransform (Transformation|GetWorldTransform (Variables|Default|GetSkeletalMesh)))
          (Development|PrintString "5"))))))

(fn ConstructionScript)