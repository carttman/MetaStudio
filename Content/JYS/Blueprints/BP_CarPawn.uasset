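; BP_CarPawn is a car pawn Blueprint with an unfinished keyboard movement setup.
; W, A and D set forward, left and right flags while held; nothing here sets the backward flag.
; Logic to turn those flags into yaw-relative AddMovementInput calls exists but is disconnected, and Tick is empty.
; As a result, key presses only update flags and this graph applies no movement.
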(event EventBeginPlay)

(event Collision|EventActorBeginOverlap
  (params (OtherActor :type Actor%20Object%20Reference)))

(event EventTick
  (params (DeltaSeconds :type Float%20%28single-precision%29)))

(event Input|KeyboardEvents|DebugKeyD
  (params (Key :type Key%20Structure :default "None") (ActionValue :type Input%20Action%20Value%20Structure)))

(event Input|KeyboardEvents|W
  (params (Key :type Key%20Structure :default "None"))
  (:Pressed
    (Variables|Default|SetisForward true))
  (:Released
    (Variables|Default|SetisForward false)))

(event Input|KeyboardEvents|D
  (params (Key :type Key%20Structure :default "None"))
  (:Pressed
    (Variables|Default|SetisRight true))
  (:Released
    (Variables|Default|SetisRight false)))

(event Input|KeyboardEvents|A
  (params (Key :type Key%20Structure :default "None"))
  (:Pressed
    (Variables|Default|SetisLeft true))
  (:Released
    (Variables|Default|SetisLeft false)))

(fn ConstructionScript)