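; Player Blueprint with an auto-focusing record camera and test hotkeys for uploading videos to Firebase.
; A looping timer from BeginPlay runs AutoDOF, which traces forward from RecordCamera and writes the hit distance into its depth-of-field post-process settings.
; Key 9 logs in anonymously through FirebaseComponent; key 0 opens an mp4 file dialog and uploads the chosen file.
; UdateFocalDistance is an uncalled alternative focus calculation, alongside disconnected cube-spawning and trace experiments.
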(event Custom|UdateFocal%20Distance
  (bind _recordcamera (Variables|Default|GetRecordCamera))
  (bind _returnvalue (Transformation|GetWorldLocation _recordcamera))
  (bind (_outhit _returnvalue_2) (Collision|LineTraceByChannel _returnvalue (+ _returnvalue (* (Math|Vector|GetForwardVector _recordcamera) 1e+04)) "TraceTypeQuery1" false 0 "None"))
  (Variables|Default|SetFocal%20Distance (Math|Float|SelectFloat (/ (Math|Vector|VectorLength (- (.Location (Collision|BreakHitResult _outhit)) (Transformation|GetWorldLocation (Variables|Default|GetRecordCamera)))) 3.0) 1e+10 _returnvalue_2)))

(event Custom|AutoDOF
  (bind _recordcamera (Variables|Default|GetRecordCamera))
  (bind _returnvalue (Transformation|GetWorldLocation _recordcamera))
  (bind (_outhit _returnvalue_2) (Collision|LineTraceByChannel _returnvalue (+ _returnvalue (* (Math|Vector|GetForwardVector _recordcamera) 3e+05)) "TraceTypeQuery1" false 0 "None"))
  (if _returnvalue_2
    (Variables|Default|SetFocus%20Location (Math|Vector|VectorLength (- (.Location (Collision|BreakHitResult _outhit)) (Transformation|GetWorldLocation (Variables|Default|GetRecordCamera)))))
    (Variables|/Script/Engine.CameraComponent|SetPostProcessSettings (Variables|Default|GetRecordCamera) (Utilities|Struct|MakePostProcessSettings 1.0 11.0 (Variables|Default|GetFocus%20Location)))))

(event EventBeginPlay
  (Utilities|Time|SetTimerbyFunctionName 0 "AutoDOF" 0.2 true)
  (Rendering|Material|SetMaterial (Variables|Default|GetCamera07) 0 0))

(event Collision|EventActorBeginOverlap
  (params (OtherActor :type Actor%20Object%20Reference)))

(event EventTick
  (params (DeltaSeconds :type Float%20%28single-precision%29)))

(event Input|MouseEvents|LeftMouseButton
  (params (Key :type Key%20Structure :default "None")))

(event Input|KeyboardEvents|9
  (params (Key :type Key%20Structure :default "None"))
  ;[1 1 1] 파이어베이스 로그인 시도
  (:Pressed
    (Class|FirebaseComponent|AnonymousLogin (Variables|Default|GetFirebaseComponent))))

(event Input|KeyboardEvents|0
  (params (Key :type Key%20Structure :default "None"))
  ;[1 1 1] 파일 탐색기 열고 => 파일 이름만 가져온다 => 파이어베이스에 업로드 시작
  (:Pressed
    (bind (_outfilenames _returnvalue) (Class|EFDFunctionLibrary|OpenFileDialog "Test" "" "" "mp4" "Single"))
    (if _returnvalue
      (bind _returnvalue_2 (Class|FirebaseComponent|GetLine (Variables|Default|GetFirebaseComponent) (Utilities|Array|Get(acopy) _outfilenames)))
      (Class|FirebaseComponent|FileUploadtoFirebase (Variables|Default|GetFirebaseComponent) (Utilities|Array|Get(acopy) _outfilenames) _returnvalue_2))))

(fn ConstructionScript)